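; BC_FadeIn is a camera system Blueprint that runs a configurable screen fade on player 0's camera manager.
; When FadeIn is enabled, BC_FadeInSetting holds a full manual fade in the pre-fade color for PreFadeTime.
; It then starts a timed fade with configurable alpha range, color, audio and hold options.
; After FadeTime it stops the fade, clearing it even if HoldWhenFinished is set.
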(event `BC_FadeInSetting`
  (bind _returnvalue (`GameplayStatics.GetPlayerCameraManager` 0))
  (bind (_fadefromalpha_x_toalpha_y__x _fadefromalpha_x_toalpha_y__y) (`KismetMathLibrary.BreakVector2D` (`self.FadeFromAlpha(X)ToAlpha(Y)`)))
  (bind _fadetime (`self.FadeTime`))
  (if (`self.FadeIn?`)
    (`PlayerCameraManager.SetManualCameraFade` (`GameplayStatics.GetPlayerCameraManager` 0) 1.0 (`self.PreFadeColor`) (`self.PreInShouldFadeAudio`))
    (`KismetSystemLibrary.Delay` (`self.PreFadeTime`))
    (`PlayerCameraManager.StartCameraFade` _returnvalue _fadefromalpha_x_toalpha_y__x _fadefromalpha_x_toalpha_y__y _fadetime (`self.FadeColor`) (`self.Should Fade Audio?`) (`self.Hold when Finished?`))
    (`KismetSystemLibrary.Delay` _fadetime)
    (`PlayerCameraManager.StopCameraFade` _returnvalue)))