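; Fixed-position zone camera in the USCS camera system that takes the view with a configurable blend while the player is inside its influence volume.
; Overlap events and DoOnce gates coordinate handoffs with the Camera, CameraCharacter and UscsForCamera Blueprints.
; Tick optionally tracks the player with clamped, interpolated look-at rotation, offset by optional manual axis input.
; The construction script selects the billboard sprite.
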(event `self.K2_OnBecomeViewTarget`
  (params (PC :type "PlayerController Object Reference"))
  (`SceneComponent.K2_SetWorldRotation` (`self.StaticCamera`) (`self.InitialRotation`) false false)
  (`/Game/CameraSystem/USCS/Blueprints/DataLibrary/BPFL_USCS_Functions.EnableControllerInput` true self))

(event `self.ReceiveBeginPlay`
  (set `self.InitialRotation` (`SceneComponent.K2_GetComponentRotation` (`self.StaticCamera`)))
  (bind _outactors (`GameplayStatics.GetAllActorsOfClass` "/Game/CameraSystem/USCS/Blueprints/SystemForCamera/BP_CameraBP.BP_CameraBP_C"))
  (set `self.CameraBP_Ref` _outactors)
  (bind _outactors_2 (`GameplayStatics.GetAllActorsOfClass` "/Game/CameraSystem/USCS/Blueprints/SystemForCamera/BP_Camera-CharacterBP.BP_Camera-CharacterBP_C"))
  (set `self.Camera-CharacterBP_Ref` _outactors_2)
  (bind _outactors_3 (`GameplayStatics.GetAllActorsOfClass` "/Game/CameraSystem/USCS/Blueprints/SystemForCamera/BP_USCS_ForCameraBP.BP_USCS_ForCameraBP_C"))
  (set `self.UscsForCameraBP_Ref` _outactors_3)
  (set `self.IsOveralpingUscsBP` false)
  (`KismetSystemLibrary.Delay` 0.01)
  (if (`PrimitiveComponent.IsOverlappingActor` (`self.StaticCameraZoneInfluencer`) (`/Game/CameraSystem/USCS/Blueprints/DataLibrary/BPFL_USCS_Functions.GetPlayerType(PawnOrCharacter)`))
    (`/Engine/EditorBlueprintResources/StandardMacros.DoOnce` false :!label _label
      (:`Completed`
        (`self.SetActorTickEnabled` true)
        (set `self.IsOveralpingUscsBP` false)
        (for _array_element (`self.Camera-CharacterBP_Ref`)
          (`/Game/CameraSystem/USCS/Blueprints/DataLibrary/BPi_USCS.BackToCamera-StaticBP` _array_element)
          (for _array_element_2 (`self.UscsForCameraBP_Ref`)
            (`/Game/CameraSystem/USCS/Blueprints/SystemForCamera/BP_USCS_ForCameraBP.BackToCamera-StaticBP` _array_element_2)
            (for _array_element_3 (`self.CameraBP_Ref`)
              (`/Game/CameraSystem/USCS/Blueprints/DataLibrary/BPi_USCS.BackToCamera-StaticBP` _array_element_3))))))))

(event `/Game/CameraSystem/USCS/Blueprints/DataLibrary/BPi_USCS.BackToUscs`
  (set `self.IsOveralpingUscsBP` true))

(event `self.StaticCameraZoneInfluencer.OnComponentBeginOverlap`
  (params (OverlappedComponent :type "PrimitiveComponent Object Reference") (OtherActor :type "Actor Object Reference") (OtherComp :type "PrimitiveComponent Object Reference") (OtherBodyIndex :type Integer) (bFromSweep :type Boolean) (SweepResult :type "HitResult Structure (by ref)"))
  (`/Game/CameraSystem/USCS/Blueprints/DataLibrary/BP_USCS_Macros.IsplayerCharacter/Pawn?` OtherActor
    (:`true`
      (goto _label))))

(event `self.StaticCameraZoneInfluencer.OnComponentEndOverlap`
  (params (OverlappedComponent :type "PrimitiveComponent Object Reference") (OtherActor :type "Actor Object Reference") (OtherComp :type "PrimitiveComponent Object Reference") (OtherBodyIndex :type Integer))
  (`/Game/CameraSystem/USCS/Blueprints/DataLibrary/BP_USCS_Macros.IsplayerCharacter/Pawn?` OtherActor
    (:`true`
      (`|ExecutionSequence`
        (:`then_0`
          (goto _label :!via `Reset`))
        (:`then_1`
          (for _array_element (`self.UscsForCameraBP_Ref`)
            (set `/Game/CameraSystem/USCS/Blueprints/SystemForCamera/BP_USCS_ForCameraBP.PreviousZoneInfluWasA_UscsZoneInflu` false _array_element)
            (goto _label_5 :!via `Reset`)))))))

(event `/Game/CameraSystem/USCS/Blueprints/DataLibrary/BPi_USCS.BackToCamera-CharacterBP`
  (`self.SetActorTickEnabled` false :!label _label_2)
  (`|ExecutionSequence`
    (:`then_0`
      (goto _label :!via `Reset`))
    (:`then_1`
      (`KismetSystemLibrary.Delay` 0.01 :!label _label_3)
      (goto _label_6 :!via `Reset`))))

(event `self.K2_OnEndViewTarget`
  (params (PC :type "PlayerController Object Reference"))
  (goto _label_2))

(event `self.ReceiveTick`
  (params (DeltaSeconds :type "Float (single-precision)"))
  (bind (_clampslopel_r_x _clampslopel_r_y) (`KismetMathLibrary.BreakVector2D` (`self.ClampSlopeL/R`)))
  (bind (_clampangledown_up_x _clampangledown_up_y) (`KismetMathLibrary.BreakVector2D` (`self.ClampAngleDown/Up`)))
  (bind (_clampanglel_r_x _clampanglel_r_y) (`KismetMathLibrary.BreakVector2D` (`self.ClampAngleL/R`)))
  (bind _staticcamera (`self.StaticCamera`))
  (bind (_returnvalue_roll _returnvalue_pitch _returnvalue_yaw) (`KismetMathLibrary.BreakRotator` (`KismetMathLibrary.FindLookAtRotation` (`SceneComponent.K2_GetComponentLocation` _staticcamera) (`self.K2_GetActorLocation` (`/Game/CameraSystem/USCS/Blueprints/DataLibrary/BPFL_USCS_Functions.GetPlayerType(PawnOrCharacter)`)))))
  (if (`self.TrackingPlayer`)
    (`SceneComponent.K2_SetWorldRotation` _staticcamera (`KismetMathLibrary.RInterpTo` (`SceneComponent.K2_GetComponentRotation` _staticcamera) (`KismetMathLibrary.MakeRotator` (`KismetMathLibrary.FClamp` _returnvalue_roll _clampslopel_r_x _clampslopel_r_y) (- (`KismetMathLibrary.FClamp` _returnvalue_pitch _clampangledown_up_x _clampangledown_up_y) (`self.RotateCameraV`)) (+ (`KismetMathLibrary.FClamp` _returnvalue_yaw _clampanglel_r_x _clampanglel_r_y) (`self.RotateCameraH`))) (`GameplayStatics.GetWorldDeltaSeconds`) (`self.InterpSpeedRotation`)) false false))
  (if (`self.IsOveralpingUscsBP`)
    (`|ExecutionSequence`
      (:`then_0`
        (`/Engine/EditorBlueprintResources/StandardMacros.DoOnce` false :!label _label_4
          (:`Completed`
            (`self.SetActorTickEnabled` false)
            (`KismetSystemLibrary.Delay` 0.01)
            (`/Game/CameraSystem/USCS/Blueprints/DataLibrary/BPFL_USCS_Functions.EnableControllerInput` false self)
            (set `self.IsOveralpingUscsBP` false)
            (`/Engine/EditorBlueprintResources/StandardMacros.DoOnce` false :!label _label_5
              (:`Completed`
                (for _array_element (`self.UscsForCameraBP_Ref`)
                  (set `/Game/CameraSystem/USCS/Blueprints/SystemForCamera/BP_USCS_ForCameraBP.PreviousZoneInfluWasA_UscsZoneInflu` true _array_element)
                  (for _array_element_2 (`self.CameraBP_Ref`)
                    (`/Game/CameraSystem/USCS/Blueprints/DataLibrary/BPi_USCS.BackToCameraBP` _array_element_2))))))))
      (:`then_1`
        (goto _label_3)))
    (else
      (`|ExecutionSequence`
        (:`then_0`
          (if (`PrimitiveComponent.IsOverlappingActor` (`self.StaticCameraZoneInfluencer`) (`/Game/CameraSystem/USCS/Blueprints/DataLibrary/BPFL_USCS_Functions.GetPlayerType(PawnOrCharacter)`))
            (`/Engine/EditorBlueprintResources/StandardMacros.DoOnce` false :!label _label_6
              (:`Completed`
                (`PlayerController.SetViewTargetWithBlend` (`GameplayStatics.GetPlayerController` 0) self (`self.Blend:TimeFromOtherCamera`) (`self.Blend:Function`) (`self.Blend:CurveShape`) (`self.Blend:Lock Outgoing`))))
            (else
              (goto _label_3))))
        (:`then_1`
          (`KismetSystemLibrary.Delay` 0.01)
          (goto _label_4 :!via `Reset`))))))

(event `InputAxis|ManualRotateCameraH`
  (params (AxisValue :type "Float (single-precision)"))
  (bind _returnvalue (`KismetMathLibrary.FClamp` AxisValue (/ (`self.AngleMinH`) 360.0) (/ (`self.AngleMaxH`) 360.0)))
  (bind _returnvalue_2 (* 360 _returnvalue))
  (bind _returnvalue_3 (* -3600 _returnvalue))
  (if (`self.CanControlCameraRotationH?`)
    (if (`self.ReverseControllerAxisH?`)
      (if (== (`self.InterpSpeedRotation`) 0.0)
        (set `self.RotateCameraH` (`KismetMathLibrary.FInterpTo` (`self.RotateCameraH`) _returnvalue_3 (`GameplayStatics.GetWorldDeltaSeconds`) (`self.SmoothControllerRotation`)))
        (else
          (set `self.RotateCameraH` _returnvalue_3)))
      (elif (== (`self.InterpSpeedRotation`) 0.0)
        (set `self.RotateCameraH` (`KismetMathLibrary.FInterpTo` (`self.RotateCameraH`) _returnvalue_2 (`GameplayStatics.GetWorldDeltaSeconds`) (`self.SmoothControllerRotation`)))
        (else
          (set `self.RotateCameraH` _returnvalue_2))))))

(event `InputAxis|ManualRotateCameraV`
  (params (AxisValue :type "Float (single-precision)"))
  (bind _returnvalue (`KismetMathLibrary.FClamp` AxisValue (/ (`self.AngleMinV:`) 360.0) (/ (`self.AngleMaxV:`) 360.0)))
  (bind _returnvalue_2 (* -360 _returnvalue))
  (bind _returnvalue_3 (* 360 _returnvalue))
  (if (`self.CanControlCameraRotationV?`)
    (if (`self.ReverseControllerAxisV?`)
      (if (== (`self.InterpSpeedRotation`) 0.0)
        (set `self.RotateCameraV` (`KismetMathLibrary.FInterpTo` (`self.RotateCameraV`) _returnvalue_2 (`GameplayStatics.GetWorldDeltaSeconds`) (`self.SmoothControllerRotation`)))
        (else
          (set `self.RotateCameraV` _returnvalue_2)))
      (elif (== (`self.InterpSpeedRotation`) 0.0)
        (set `self.RotateCameraV` (`KismetMathLibrary.FInterpTo` (`self.RotateCameraV`) _returnvalue_3 (`GameplayStatics.GetWorldDeltaSeconds`) (`self.SmoothControllerRotation`)))
        (else
          (set `self.RotateCameraV` _returnvalue_3))))))

(fn `UserConstructionScript`
  (bind _spritecollection (`self.SpriteCollection`))
  (bind _returnvalue (`KismetMathLibrary.Clamp` (`self.ThumnailSelector:`) 0 (- (`KismetArrayLibrary.Array_Length` _spritecollection) 1)))
  (set `self.ThumnailSelector:` _returnvalue)
  (set `BillboardComponent.Sprite` (`|GetArrayItem` _spritecollection _returnvalue) (`self.Billboard`)))