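; H-8 Extension actor that smoothly turns to face the player character while the player overlaps its Sphere component.
; BeginPlay caches the player character and starts a self-calling Delay loop that polls the overlap and sets a ShouldRotate flag.
; FacePlayer interpolates toward the look-at rotation and re-calls itself while the flag holds.
; Each overlapping poll also calls FacePlayer again, alongside its own loop.
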(event `self.ReceiveBeginPlay`
  (bind _asbp_third_person_character (cast `/Game/ThirdPerson/Blueprints/BP_ThirdPersonCharacter` (`GameplayStatics.GetPlayerCharacter` 0))
    (:`then`
      (set `self.As BP Third Person Character` _asbp_third_person_character)
      (`self.Should Rotate ?`))
    (:`CastFailed`
      (`KismetSystemLibrary.PrintString` "Hello"))))

(event `Face Player`
  (bind (_returnvalue_roll _returnvalue_pitch _returnvalue_yaw) (`KismetMathLibrary.BreakRotator` (`KismetMathLibrary.RInterpTo` (`self.K2_GetActorRotation`) (`KismetMathLibrary.FindLookAtRotation` (`self.K2_GetActorLocation`) (`self.K2_GetActorLocation` (`self.As BP Third Person Character`))) (`GameplayStatics.GetWorldDeltaSeconds`) 1.0)))
  (if (`self.ShouldRotate?`)
    (`self.K2_SetActorRotation` (`KismetMathLibrary.MakeRotator` _returnvalue_roll _returnvalue_pitch _returnvalue_yaw))
    (`KismetSystemLibrary.Delay` 0.001)
    (`self.Face Player`)))

(event `Should Rotate ?`
  (if (`PrimitiveComponent.IsOverlappingActor` (`self.Sphere`) (`self.As BP Third Person Character`))
    (set `self.ShouldRotate?` true)
    (`self.Face Player`)
    (else
      (set `self.ShouldRotate?` false)))
  (`KismetSystemLibrary.Delay` 0.001)
  (`self.Should Rotate ?`))

(fn `UserConstructionScript`)