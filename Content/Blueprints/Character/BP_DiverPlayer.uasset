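; BP_DiverPlayer is the player diver character, which swims relative to the camera's control rotation.
; BeginPlay adds the IMC_Structure Enhanced Input context; IA_Swim and IA_SwimPitch then move the actor along control forward and up via swept SetActorLocation, scaled by MovementSpeed but not delta time.
; Only IA_Swim turns the body, interpolating toward the combined input direction.
; Both inputs fire CallOnCharacterStop while triggered and CallOnCharacterMoving on completion, opposite to their names.
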(event `self.ReceiveBeginPlay`
  (bind _asplayer_controller (cast `PlayerController` (`self.GetController`)))
  (bind _returnvalue (pcsubsystem `EnhancedInputLocalPlayerSubsystem` _asplayer_controller))
  (`/Engine/EditorBlueprintResources/StandardMacros.IsValid` _returnvalue
    (:`Is Valid`
      (`EnhancedInputSubsystemInterface.AddMappingContext` _returnvalue "/Game/ThirdPerson/Inputs/IMC_Structure.IMC_Structure" 0 (struct)))))

(event `EnhancedInput|/Game/ThirdPerson/Inputs/IA_Swim`
  (params (ActionValue :type "Vector2D Structure") (ElapsedSeconds :type "Float (double-precision)") (TriggeredSeconds :type "Float (double-precision)") (InputAction :type "InputAction Object Reference" :default "/Game/ThirdPerson/Inputs/IA_Swim.IA_Swim"))
  (bind _returnvalue (`KismetMathLibrary.GetForwardVector` (`self.GetControlRotation`)))
  ;[1 1 1] Player Movement
  (:`Triggered`
    (`self.OnCharacterStop`)
    (bind _output_get (set `self.MoveRight` ActionValue_X))
    (`self.K2_SetActorLocation` (+ (`self.K2_GetActorLocation`) (* _returnvalue (/ _output_get 50.0) (`self.MovementSpeed`))) true)
    (`self.K2_SetActorRotation` (`KismetMathLibrary.RInterpTo` (`self.K2_GetActorRotation`) (`KismetMathLibrary.MakeRotFromX` (`KismetMathLibrary.Normal` (+ (* _returnvalue _output_get) (* (`KismetMathLibrary.GetUpVector` (`self.GetControlRotation`)) (stale `EnhancedInput|/Game/ThirdPerson/Inputs/IA_SwimPitch` _output_get))))) (`GameplayStatics.GetWorldDeltaSeconds`) 10.0) true))
  (:`Completed`
    (`self.OnCharacterMoving`)))

(event `EnhancedInput|/Game/ThirdPerson/Inputs/IA_SwimPitch`
  (params (ActionValue :type "Vector2D Structure") (ElapsedSeconds :type "Float (double-precision)") (TriggeredSeconds :type "Float (double-precision)") (InputAction :type "InputAction Object Reference" :default "/Game/ThirdPerson/Inputs/IA_SwimPitch.IA_SwimPitch"))
  ;[1 1 1] Player Movement
  (:`Triggered`
    (`self.OnCharacterStop`)
    (bind _output_get (set `self.MoveUp` ActionValue_X))
    (`self.K2_SetActorLocation` (+ (* (`KismetMathLibrary.GetUpVector` (`self.GetControlRotation`)) (/ _output_get 50.0) (`self.MovementSpeed`)) (`self.K2_GetActorLocation`)) true))
  (:`Completed`
    (`self.OnCharacterMoving`)))

(fn `UserConstructionScript`)