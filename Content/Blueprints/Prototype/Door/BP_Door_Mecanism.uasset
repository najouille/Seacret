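; Prototype door mechanism that slides or rotates a target actor, ItemToMove, through a trigger volume.
; Begin and end overlaps wait a delay, guarded by IsMoving, then drive timelines via Location and Rotate graphs.
; Slide mode opens on entry and reverses on exit if CloseEnable; rotate mode turns toward NewRotation only on exit.
; Overlaps only check that the player or ItemToActivateDoor is valid, not which actor overlapped.
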(event `self.CollisionComponent.OnComponentEndOverlap`
  (params (OverlappedComponent :type "PrimitiveComponent Object Reference") (OtherActor :type "Actor Object Reference") (OtherComp :type "PrimitiveComponent Object Reference") (OtherBodyIndex :type Integer))
  (if (or (`KismetSystemLibrary.IsValid` (`GameplayStatics.GetPlayerCharacter` 0)) (`KismetSystemLibrary.IsValid` (`self.ItemToActivateDoor`)))
    (set `self.isEnable?` false)
    (`KismetSystemLibrary.PrintString` "Disable")
    (if (not (`self.isMoving`))
      (set `self.isMoving` true)
      (`KismetSystemLibrary.Delay` (`self.Duration`))
      (if (`self.FalseL/TrueR`)
        (bind (_direction _newtrack_0) (`Timeline|Timeline_Rotation`)
          (:`Update`
            (`self.K2_SetActorRotation` (`self.ItemToMove`) (`KismetMathLibrary.RLerp` (`self.K2_GetActorRotation` (`self.ItemToMove`)) (`self.New Rotation`) _newtrack_0) false)
            (set `self.isMoving` false)))
        (elif (`self.CloseEnable`)
          (bind (_direction_2 _newtrack_0_2) (`Timeline|Timeline_Location_Open` :!via `Reverse` :!label _label)
            (:`Update`
              (`self.K2_SetActorLocation` (`self.ItemToMove`) (`KismetMathLibrary.VLerp` (`self.Close Location`) (`self.Open Location`) _newtrack_0_2) false false)
              (set `self.isMoving` false))))))))

(event `self.CollisionComponent.OnComponentBeginOverlap`
  (params (OverlappedComponent :type "PrimitiveComponent Object Reference") (OtherActor :type "Actor Object Reference") (OtherComp :type "PrimitiveComponent Object Reference") (OtherBodyIndex :type Integer) (bFromSweep :type Boolean) (SweepResult :type "HitResult Structure (by ref)"))
  (if (or (`KismetSystemLibrary.IsValid` (`GameplayStatics.GetPlayerCharacter` 0)) (`KismetSystemLibrary.IsValid` (`self.ItemToActivateDoor`)))
    (set `self.isEnable?` true)
    (`KismetSystemLibrary.PrintString` "Enable")
    (if (not (`self.isMoving`))
      (set `self.isMoving` true)
      (`KismetSystemLibrary.Delay` (`self.Duration`))
      (if (`self.FalseL/TrueR`)
        (set `self.isMoving` false)
        (else
          (goto _label))))))

(fn `UserConstructionScript`)