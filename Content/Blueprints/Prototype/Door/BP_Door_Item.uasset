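; Prototype sliding door that moves a cube between two points, PointA and PointB, when interacted with or triggered by a lever.
; Each interaction flips the target point, starts movement and switches an LED between green and red materials.
; Tick moves the cube at constant speed toward the target until it is within a small distance.
; The lever event also reverses the door again after a timer delay.
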(event `self.ReceiveBeginPlay`)

(event `self.ReceiveTick`
  (params (DeltaSeconds :type "Float (single-precision)"))
  (bind _returnvalue (`SceneComponent.K2_GetComponentLocation` (`self.Point A`)))
  (bind _returnvalue_2 (`SceneComponent.K2_GetComponentLocation` (`self.Cube`)))
  (bind _returnvalue_3 (`SceneComponent.K2_GetComponentLocation` (`self.Point B`)))
  (bind _returnvalue_4 (`SceneComponent.K2_GetComponentLocation` (`self.Cube`)))
  (if (`self.b_IsMoving`)
    (if (`self.CurrentPoint`)
      (`KismetSystemLibrary.PrintString` "s'ouvre")
      (`SceneComponent.K2_AddWorldOffset` (`self.Cube`) (* (`KismetMathLibrary.Normal` (- _returnvalue_3 _returnvalue_4)) DeltaSeconds (`self.Speed`)) false false)
      (if (not (> (`KismetMathLibrary.Vector_Distance` _returnvalue_3 _returnvalue_4) 5.0))
        (set `self.b_IsMoving` false))
      (else
        (`KismetSystemLibrary.PrintString` "se ferme")
        (`SceneComponent.K2_AddWorldOffset` (`self.Cube`) (* (`KismetMathLibrary.Normal` (- _returnvalue _returnvalue_2)) DeltaSeconds (`self.Speed`)) false false)
        (if (not (> (`KismetMathLibrary.Vector_Distance` _returnvalue _returnvalue_2) 5.0))
          (set `self.b_IsMoving` false))))))

(event `/Game/Blueprints/BPI_ButtonTarget.OnInteract`
  (bind _output_get (set `self.CurrentPoint` (== (`self.CurrentPoint`) false)))
  (set `self.b_IsMoving` true)
  (`self.ChangeMaterial` _output_get))

(event `/Game/Blueprints/BPI_ButtonTarget.OnLeverInteract`
  (params (timer :type "Float (double-precision)"))
  (bind _output_get (set `self.CurrentPoint` (== (`self.CurrentPoint`) false)))
  (set `self.b_IsMoving` true)
  (`self.ChangeMaterial` _output_get)
  (`KismetSystemLibrary.Delay` timer)
  (bind _output_get_2 (set `self.CurrentPoint` (== (`self.CurrentPoint`) false)))
  (set `self.b_IsMoving` true)
  (`self.ChangeMaterial` _output_get_2))

(fn `ChangeMaterial`
  (params (Material :type Boolean))
  (bind _led (`self.LED`))
  (if Material
    (`PrimitiveComponent.SetMaterial` _led 0 "/Game/Materials/Prototype/Button/M_Green.M_Green")
    (else
      (`PrimitiveComponent.SetMaterial` _led 0 "/Game/Materials/Prototype/Button/M_Red.M_Red"))))

(fn `UserConstructionScript`)