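; BP_Button is a prototype button that shows whether a door mechanism is enabled by the color of its box.
; On BeginPlay it gathers all BP_Door_Mecanism actors, casts the one at a hard-coded array index, stores it and prints the cast result.
; Every Tick it polls that door's IsEnable flag and sets the box material to green or red.
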(event `self.ReceiveBeginPlay`
  (bind _outactors (`GameplayStatics.GetAllActorsOfClass` "/Game/Blueprints/Prototype/Door/BP_Door_Mecanism.BP_Door_Mecanism_C"))
  (bind _asbp_door_mecanism (cast `/Game/Blueprints/Prototype/Door/BP_Door_Mecanism` (`|GetArrayItem` _outactors 2))
    (:`then`
      (set `self.As BP Door Mecanism` _asbp_door_mecanism)
      (`KismetSystemLibrary.PrintString` "cast successful"))
    (:`CastFailed`
      (`KismetSystemLibrary.PrintString` "cast failed"))))

(event `self.ReceiveTick`
  (params (DeltaSeconds :type "Float (single-precision)"))
  (bind _box (`self.Box`))
  (if (`/Game/Blueprints/Prototype/Door/BP_Door_Mecanism.isEnable?` (`self.As BP Door Mecanism`))
    (`PrimitiveComponent.SetMaterial` _box 0 "/Game/Materials/Prototype/Button/M_Green.M_Green")
    (else
      (`PrimitiveComponent.SetMaterial` _box 0 "/Game/Materials/Prototype/Button/M_Red.M_Red"))))

(fn `UserConstructionScript`)