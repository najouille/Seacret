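; Interactable puzzle box actor that can be pulled toward a player location passed in by its caller.
; Each Pull call moves it by Speed times delta time with a swept offset, applying the world-space direction as a local offset.
; It prints the remaining distance and returns whether the box is within a fixed threshold of that location.
; The event graph and construction script are empty.
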(fn `Pull`
  (params (PlayerLocation :type "Vector Structure"))
  (returns (PullFinished :type Boolean))
  (bind _returnvalue (`self.K2_GetActorLocation`))
  (bind _returnvalue_2 (`KismetMathLibrary.Vector_Distance` PlayerLocation _returnvalue))
  (`self.K2_AddActorLocalOffset` (* (`KismetMathLibrary.Normal` (- PlayerLocation _returnvalue)) (`GameplayStatics.GetWorldDeltaSeconds`) (`self.Speed`)) true)
  (`KismetSystemLibrary.PrintString` (`KismetStringLibrary.Conv_DoubleToString` _returnvalue_2))
  (return (< _returnvalue_2 100.0)))

(fn `UserConstructionScript`)