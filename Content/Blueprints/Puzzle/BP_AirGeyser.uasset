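; Toggleable air geyser puzzle hazard that kills players and drives interactable objects caught in its stream.
; While active, it line-traces from its base to DestPoint every tick, calling Die on players or sending other actors that point and its active state.
; It toggles by interaction or a recursive delay cycle; levers start a timed run where a timeline scales GeyserDistance, then shuts it off.
; Older player-push logic remains disconnected.
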(event `self.ReceiveBeginPlay`
  (bind _ns_airflow (`self.NS_AirFlow`))
  (if (`self.b_IsSequential`)
    (`KismetSystemLibrary.Delay` (`self.Delay Before Starting`))
    (`self.Sequential`))
  (set `self.GeyserDistance` (`self.GeyserDistanceBase`))
  (if (`self.Activated`)
    (`ActorComponent.Activate` _ns_airflow false)
    (else
      (`ActorComponent.Deactivate` _ns_airflow))))

(event `/Game/Blueprints/BPI_ButtonTarget.OnInteract`
  (bind _returnvalue (`self.DestPoint`))
  (bind _ns_airflow (`self.NS_AirFlow`))
  (bind _output_get (set `self.Activated` (== (`self.Activated`) false)))
  (if _output_get
    (`ActorComponent.Activate` _ns_airflow false)
    (else
      (`ActorComponent.Deactivate` _ns_airflow :!label _label)))
  (bind (_outhit _returnvalue_2) (`KismetSystemLibrary.LineTraceSingle` :`Start` (`SceneComponent.K2_GetComponentLocation` (`self.Socle`)) :`End` _returnvalue :`TraceChannel` "TraceTypeQuery1" :`DrawDebugType` "ForOneFrame" :!label _label_2))
  (if _returnvalue_2
    (bind (_bblockinghit _binitialoverlap _time _distance _location _impactpoint _normal _impactnormal _physmat _hitactor) (`GameplayStatics.BreakHitResult` _outhit))
    (if (`self.ActorHasTag` _hitactor "Player")
      (bind _asbp_third_person_character (cast `/Game/ThirdPerson/Blueprints/BP_ThirdPersonCharacter` _hitactor))
      (`/Game/ThirdPerson/Blueprints/BP_ThirdPersonCharacter.Die` _asbp_third_person_character)
      (else
        (message `/Game/Blueprints/BPI_HarpoonInteractable.OnInteract` _hitactor _returnvalue (`self.Activated`))))))

(event `self.ReceiveTick`
  (params (DeltaSeconds :type "Float (single-precision)"))
  (if (`self.Activated`)
    (goto _label_2)))

(event `Sequential`
  (if (`self.Activated`)
    (`KismetSystemLibrary.PrintString` "je m'active")
    (`/Game/Blueprints/BPI_ButtonTarget.OnInteract`)
    (`KismetSystemLibrary.Delay` (`self.TimeOn`))
    (else
      (`KismetSystemLibrary.PrintString` "Je me desactive")
      (`/Game/Blueprints/BPI_ButtonTarget.OnInteract`)
      (`KismetSystemLibrary.Delay` (`self.TimeOff`))))
  (`self.Sequential`))

(event `/Game/Blueprints/BPI_ButtonTarget.OnLeverInteract`
  (params (timer :type "Float (double-precision)"))
  (bind _ns_airflow (`self.NS_AirFlow`))
  (`TimelineComponent.SetPlayRate` (`self.IntensityTimer`) (/ 1.0 timer))
  (bind _output_get (set `self.Activated` (== (`self.Activated`) false)))
  (if _output_get
    (`ActorComponent.Activate` _ns_airflow false)
    (bind (_direction _intensity) (`Timeline|IntensityTimer` :!via `PlayFromStart`)
      (:`Update`
        (set `self.GeyserDistance` (* (`self.GeyserDistanceBase`) _intensity)))
      (:`Finished`
        (set `self.Activated` false)
        (goto _label)))
    (else
      (`ActorComponent.Deactivate` _ns_airflow)
      (goto _label_2))))

(fn `GetGeyserDistance`
  (returns (GeyserDistance :type "Float (double-precision)"))
  (return (`self.GeyserDistance`)))

(fn `SetGeyserDistance`
  (params (GeyserDistance :type "Float (double-precision)"))
  (set `self.GeyserDistance` GeyserDistance))

(fn `UserConstructionScript`)