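; BP_FragileSurface is a puzzle actor whose Geometry Collection surface breaks when interacted with.
; OnInteract enables physics and rigid body collision notifications on GCFragileSurface, disables BoxCollision, then applies a Chaos internal cluster strain field through RadialFalloff to fracture it.
; StopInteraction is empty, and GetSpeed returns a constant.
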(event `/Game/Blueprints/BPI_HarpoonInteractable.StopInteraction`)

(event `/Game/Blueprints/BPI_HarpoonInteractable.OnInteract`
  (params (FinalPosition :type "Vector Structure") (Stay :type Boolean))
  (bind _gc_fragilesurface (`self.GC_FragileSurface`))
  (`PrimitiveComponent.SetNotifyRigidBodyCollision` _gc_fragilesurface true)
  (`PrimitiveComponent.SetSimulatePhysics` _gc_fragilesurface true)
  (`PrimitiveComponent.SetCollisionEnabled` (`self.BoxCollision`) "NoCollision")
  (`GeometryCollectionComponent.ApplyPhysicsField` (`self.GC_FragileSurface`) false "Chaos_InternalClusterStrain" null (`self.RadialFalloff`)))

(fn `GetSpeed`
  (returns (Speed :type "Float (double-precision)"))
  (return 1000.0))

(fn `UserConstructionScript`)